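; BP_Crop is a bobbing vegetable pickup that gives the player a seed of its SeedType.
; The construction script picks the mesh, material and scale from SeedType, and a timeline drives the bob.
; Overlapping PullCollision opens a Tick gate that pulls the actor toward a point below the player's location at constant speed.
; Overlapping CollectCollision adds the seed to the player's ACSeedComponent and destroys the actor.
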(event `self.ReceiveBeginPlay`
  (bind _relativelocation (`SceneComponent.RelativeLocation` (`self.StaticMesh`)))
  (`parent.ReceiveBeginPlay`)
  (set `self.Player Seeds` (`/Game/Blueprints/BP_FirstPersonCharacter.AC_SeedComponent` (`self.Player`)))
  (bind (_direction _lerp) (`Timeline|TL_Bob`)
    (:`Update`
      (`SceneComponent.K2_SetRelativeLocation` (`self.StaticMesh`) (`KismetMathLibrary.VLerp` (- _relativelocation (0.0 0.0 0.5)) (+ _relativelocation (0.0 0.0 0.5)) _lerp) false false))))

(event `/Game/Blueprints/Interfaces/I_Interact.Interact`)

(event `self.PullCollision.OnComponentBeginOverlap`
  (params (OverlappedComponent :type "PrimitiveComponent Object Reference") (OtherActor :type "Actor Object Reference") (OtherComp :type "PrimitiveComponent Object Reference") (OtherBodyIndex :type Integer) (bFromSweep :type Boolean) (SweepResult :type "HitResult Structure (by ref)"))
  (if (== OtherActor (`self.Player`))
    (`self.MoveToPlayer`)))

(event `self.ReceiveTick`
  (params (DeltaSeconds :type "Float (single-precision)"))
  (`/Engine/EditorBlueprintResources/StandardMacros.Gate` true :!label _label
    (:`Exit`
      (`self.K2_SetActorLocation` (`KismetMathLibrary.VInterpTo_Constant` (`self.K2_GetActorLocation`) (- (`self.K2_GetActorLocation` (`self.Player`)) (0.0 0.0 80.0)) DeltaSeconds 800.0)))))

(event `MoveToPlayer`
  (goto _label :!via `Open`))

(event `self.CollectCollision.OnComponentBeginOverlap`
  (params (OverlappedComponent :type "PrimitiveComponent Object Reference") (OtherActor :type "Actor Object Reference") (OtherComp :type "PrimitiveComponent Object Reference") (OtherBodyIndex :type Integer) (bFromSweep :type Boolean) (SweepResult :type "HitResult Structure (by ref)"))
  (if (== OtherActor (`self.Player`))
    (`/Game/Blueprints/Components/AC_SeedComponent.Add Seed` (`self.Player Seeds`) (`self.SeedType`))
    (`self.K2_DestroyActor`)))

(fn `UserConstructionScript`
  (bind _seedtype (`self.SeedType`))
  (`parent.UserConstructionScript`)
  (`StaticMeshComponent.SetStaticMesh` (`self.StaticMesh`) (select `/Game/Blueprints/Enums/E_SeedTypes` _seedtype :`NewEnumerator0` "/Game/GreenwoodFantasyVillage/Meshes/SM_Carrot.SM_Carrot" :`NewEnumerator2` "/Game/GreenwoodFantasyVillage/Meshes/SM_Onion.SM_Onion" :`NewEnumerator3` "/Game/Food_Pack_01/Meshes/Food_Root_Potato_01.Food_Root_Potato_01" :`NewEnumerator4` "/Game/Food_Pack_01/Meshes/Food_Root_Garlic_01.Food_Root_Garlic_01" :!type "StaticMesh Object Reference"))
  (`PrimitiveComponent.SetMaterial` (`self.StaticMesh`) 0 (select `/Game/Blueprints/Enums/E_SeedTypes` _seedtype :`NewEnumerator0` "/Game/GreenwoodFantasyVillage/Materials/MI_Vegetables.MI_Vegetables" :`NewEnumerator2` "/Game/GreenwoodFantasyVillage/Materials/MI_Vegetables.MI_Vegetables" :`NewEnumerator3` "/Game/Food_Pack_01/Materials/M_Food_Root_Potato_01.M_Food_Root_Potato_01" :`NewEnumerator4` "/Game/Food_Pack_01/Materials/M_Food_Root_Garlic_01.M_Food_Root_Garlic_01" :!type "MaterialInterface Object Reference"))
  (`SceneComponent.SetWorldScale3D` (`self.StaticMesh`) (* (`self.GetActorScale3D`) (`KismetMathLibrary.Conv_DoubleToVector` (select `/Game/Blueprints/Enums/E_SeedTypes` (`self.SeedType`) :`NewEnumerator0` 0.8 :`NewEnumerator2` 0.8 :`NewEnumerator3` 2.0 :`NewEnumerator4` 3.0 :!type "Float (single-precision)")))))