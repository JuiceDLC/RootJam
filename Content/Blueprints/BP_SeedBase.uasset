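; Base seed pickup actor that adds its seed type to the player's inventory when interacted with.
; The construction script uses the SeedType enum to set the display name and sphere material, though only the carrot has a material assigned.
; BeginPlay caches the first-person character's ACSeedComponent, and Interact calls AddSeed on it, prints a debug message, then destroys the actor.
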(event `self.ReceiveBeginPlay`
  (bind _asbp_first_person_character (cast `/Game/Blueprints/BP_FirstPersonCharacter` (`GameplayStatics.GetPlayerCharacter` 0)))
  (bind _output_get (set `self.Player` _asbp_first_person_character))
  (set `self.Player Seeds` (`/Game/Blueprints/BP_FirstPersonCharacter.AC_SeedComponent` _output_get)))

(event `/Game/Blueprints/Interfaces/I_Interact.Interact`
  (`KismetSystemLibrary.PrintString` "Interacted")
  (`/Game/Blueprints/Components/AC_SeedComponent.Add Seed` (`self.Player Seeds`) (`self.SeedType`))
  (`self.K2_DestroyActor`))

(fn `UserConstructionScript`
  (`PrimitiveComponent.SetMaterial` (`self.Sphere`) 0 (select `/Game/Blueprints/Enums/E_SeedTypes` (`self.SeedType`) :`NewEnumerator0` "/Game/LevelPrototyping/Materials/MI_Solid_Orange.MI_Solid_Orange" :!type "MaterialInterface Object Reference"))
  (set `self.SeedName` (select `/Game/Blueprints/Enums/E_SeedTypes` (`self.SeedType`) :`NewEnumerator0` "Carrot" :`NewEnumerator2` "Onion" :`NewEnumerator3` "Potato" :`NewEnumerator4` "Radish")))