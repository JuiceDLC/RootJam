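; BP_Dirt is an interactable dirt object that lets the player open a seed selection menu.
; On BeginPlay it casts the player character to BP_FirstPersonCharacter and caches that character's seed component.
; Interact adds a new W_SeedSelect widget to the viewport when the component's total seed count is above zero, and otherwise prints a "No Seeds" message.
; ReleaseInteract and the construction script are empty.
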(event `self.ReceiveBeginPlay`
  (bind _asbp_first_person_character (cast `/Game/Blueprints/BP_FirstPersonCharacter` (`GameplayStatics.GetPlayerCharacter` 0)))
  (bind _output_get (set `self.Player` _asbp_first_person_character))
  (set `self.Player Seeds` (`/Game/Blueprints/BP_FirstPersonCharacter.AC_SeedComponent` _output_get)))

(event `/Game/Blueprints/Interfaces/I_Interact.Interact`
  (if (> (`/Game/Blueprints/Components/AC_SeedComponent.TotalSeeds` (`self.Player Seeds`)) 0)
    (bind _returnvalue (`|CreateWidget` "/Game/Widgets/W_SeedSelect.W_SeedSelect_C"))
    (`UserWidget.AddToViewport` _returnvalue 0)
    (else
      (`KismetSystemLibrary.PrintString` "No Seeds"))))

(event `/Game/Blueprints/Interfaces/I_Interact.Release Interact`)

(fn `UserConstructionScript`)