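; Roaming enemy with random ghost sounds that hunts the player, showing game over on DeathRange overlap and the win screen when its health runs out.
; It wanders between BP_NavigationPoints sorted by distance to the player, favouring the closest as the player's seed total rises.
; Damage, or a Box overlap confirmed by line trace while the player isn't Onioned, starts a chase.
; A looping timer resumes wandering once the player is far away.
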(event `Sound`
  (`GameplayStatics.PlaySoundAtLocation` "/Game/Sounds/Ghost_-_Sound_Effect.Ghost_-_Sound_Effect" (`self.K2_GetActorLocation`) (struct) 1.0 (`KismetMathLibrary.RandomFloatInRange` 0.7 1.1) 0.0 null null null null))

(event `self.ReceiveBeginPlay`
  (`self.Get References BeginPlay`)
  (`self.Navigate to Next Point`)
  (add `self.OnTakeAnyDamage` (delegate `Damage`))
  (`KismetSystemLibrary.K2_SetTimerDelegate` (delegate `Sound`) (`KismetMathLibrary.RandomFloatInRange` 15.0 45.0) true))

(event `Damage` :!signature `self.OnTakeAnyDamage`
  (params (DamagedActor :type "Actor Object Reference") (Damage :type "Float (single-precision)") (DamageType :type "DamageType Object Reference") (InstigatedBy :type "Controller Object Reference") (DamageCauser :type "Actor Object Reference"))
  (`/Engine/EditorBlueprintResources/StandardMacros.DecrementFloat` (`self.Health`)
    (:`  `
      (if (<= (`self.Health`) 0.0)
        (bind _returnvalue (`|CreateWidget` "/Game/Widgets/W_Win.W_Win_C"))
        (`UserWidget.AddToViewport` _returnvalue 0)
        (else
          (set `self.State` "NewEnumerator1")
          (`self.Hunt`))))))

(event `Navigate to Next Point`
  (bind _nav_point (`self.ChooseNewLocation`))
  (bind _location (`self.Get Random Location Within Nav Point` _nav_point))
  (`AITask_MoveTo.AIMoveTo` (`AIBlueprintHelperLibrary.GetAIController` self) _location null
    (:`OnRequestFailed`
      (`KismetSystemLibrary.PrintString` "fail"))
    (:`OnMoveFinished`
      (`KismetSystemLibrary.Delay` (`self.Wait Before Moving Again`))
      (if (`|EnumEquality` (`self.State`) "NewEnumerator0")
        (`self.Navigate to Next Point`)))))

(event `Navigate to Specific Point`
  (params (Location :type "/Game/Blueprints/Enums/E_NavLocations Enum" :default "E_NavLocations_MAX"))
  (bind _navpoint (`self.Get Location Nav Point` Location))
  (bind _location (`self.Get Random Location Within Nav Point` _navpoint))
  (`AITask_MoveTo.AIMoveTo` (`AIBlueprintHelperLibrary.GetAIController` self) _location null))

(event `self.Box.OnComponentBeginOverlap`
  (params (OverlappedComponent :type "PrimitiveComponent Object Reference") (OtherActor :type "Actor Object Reference") (OtherComp :type "PrimitiveComponent Object Reference") (OtherBodyIndex :type Integer) (bFromSweep :type Boolean) (SweepResult :type "HitResult Structure (by ref)"))
  (bind _player (`self.Player`))
  (if (== OtherActor _player)
    (if (not (`/Game/Blueprints/BP_FirstPersonCharacter.Onioned` _player))
      (bind _outhit (`KismetSystemLibrary.LineTraceSingle` :`Start` (`self.K2_GetActorLocation`) :`End` (`self.K2_GetActorLocation` _player) :`TraceChannel` "TraceTypeQuery1" :`DrawDebugType` "Persistent"))
      (if (== (`.HitActor` (`GameplayStatics.BreakHitResult` _outhit)) null)
        (set `self.State` "NewEnumerator1")
        (`self.Hunt`)))))

(event `Hunt`
  (`AITask_MoveTo.AIMoveTo` (`AIBlueprintHelperLibrary.GetAIController` self) (0.0 0.0 0.0) (`self.Player`)
    (:`then`
      (bind _returnvalue (`KismetSystemLibrary.K2_SetTimerDelegate` (delegate `Check if Player is close`) 0.5 true)))))

(event `Check if Player is close`
  (if (>= (`KismetMathLibrary.VSize` (- (`self.K2_GetActorLocation`) (`self.K2_GetActorLocation` (`self.Player`)))) 3000.0)
    (set `self.State` "NewEnumerator0")
    (`self.Navigate to Next Point`)
    (`KismetSystemLibrary.K2_PauseTimerHandle` (stale `Hunt` _returnvalue))))

(event `self.DeathRange.OnComponentBeginOverlap`
  (params (OverlappedComponent :type "PrimitiveComponent Object Reference") (OtherActor :type "Actor Object Reference") (OtherComp :type "PrimitiveComponent Object Reference") (OtherBodyIndex :type Integer) (bFromSweep :type Boolean) (SweepResult :type "HitResult Structure (by ref)"))
  (if (== OtherActor (`self.Player`))
    (bind _returnvalue (`|CreateWidget` "/Game/Widgets/W_GameOver.W_GameOver_C"))
    (`UserWidget.AddToViewport` _returnvalue 0)))

(fn `ChooseNewLocation`
  (returns (`Nav Point` :type "/Game/Blueprints/BP_NavigationPoint Object Reference"))
  (locals (Distances :type "Array of Float (double-precision)") (Shortest :type "Float (double-precision)") (Longest :type "Float (double-precision)") (Median :type "Float (double-precision)") (SortedNavPoints :type "Array of /Game/Blueprints/BP_NavigationPoint Object Reference") (`Last Index` :type Integer :default 0) (`Total Seeds` :type Integer :default 0) (MaxAmountOfSeeds :type Integer :default 100) (PercentOfClose :type "Float (double-precision)") (PercentOfMedian :type "Float (double-precision)") (PercentOfFar :type "Float (double-precision)") (ReturnNav :type "/Game/Blueprints/BP_NavigationPoint Object Reference"))
  (bind _returnvalue (`KismetMathLibrary.RandomFloatInRange` 0.0 100.0))
  (bind _sortednavpoints (`self.Get Nav Distances`))
  ;[1 1 1] Save Needed Variables
  (bind _output_get (set `local.SortedNavPoints` _sortednavpoints))
  (set `local.Last Index` (`KismetArrayLibrary.Array_LastIndex` _output_get))
  (bind _output_get_2 (set `local.Total Seeds` (`/Game/Blueprints/Components/AC_SeedComponent.TotalSeeds` (`self.Player Seeds`))))
  ;[1 1 1] Calculate Percent Chances from Seed Total
  (bind _output_get_3 (set `local.PercentOfClose` (* (/ _output_get_2 (`local.MaxAmountOfSeeds`)) 100.0)))
  (bind _returnvalue_2 (/ (- 100.0 _output_get_3) 2.0))
  (bind _output_get_4 (set `local.PercentOfMedian` (+ _output_get_3 _returnvalue_2)))
  (set `local.PercentOfFar` (+ _output_get_4 _returnvalue_2))
  ;[1 1 1] Use Percent Chances to Decide which Nav Point Enemy will Move To
  (if (<= _returnvalue (`local.PercentOfClose`))
    (set `local.ReturnNav` (`|GetArrayItem` (`local.SortedNavPoints`)))
    (elif (<= _returnvalue (`local.PercentOfMedian`))
      (set `local.ReturnNav` (`|GetArrayItem` (`local.SortedNavPoints`) (/ (`local.Last Index`) 2)))
      (else
        (set `local.ReturnNav` (`|GetArrayItem` (`local.SortedNavPoints`) (`local.Last Index`))))))
  (return (`local.ReturnNav`)))

(fn `Get Location Nav Point`
  (params (Location :type "/Game/Blueprints/Enums/E_NavLocations Enum" :default "E_NavLocations_MAX"))
  (returns (NavPoint :type "/Game/Blueprints/BP_NavigationPoint Object Reference"))
  (locals (NavAtLocation :type "/Game/Blueprints/BP_NavigationPoint Object Reference"))
  (for _array_element (`self.NavPoints`)
    (if (`|EnumEquality` (`/Game/Blueprints/BP_NavigationPoint.Location` _array_element) Location)
      (set `local.NavAtLocation` _array_element)))
  (return (`local.NavAtLocation`)))

(fn `Get Nav Distances`
  (returns (SortedNavPoints :type "Array of /Game/Blueprints/BP_NavigationPoint Object Reference"))
  (locals (Distances :type "Array of Float (double-precision)") (SortedNavs :type "Array of /Game/Blueprints/BP_NavigationPoint Object Reference") (`Local Nav Points` :type "Array of /Game/Blueprints/BP_NavigationPoint Object Reference") (`For Loop Last Index` :type Integer :default 0))
  (bind _sortednavs (`local.SortedNavs`))
  (bind _indexofmaxvalue (`KismetMathLibrary.MaxOfFloatArray` (`local.Distances`)))
  ;[1 1 1] Use a local array to not mess up the main array
  (set `local.Local Nav Points` (`self.NavPoints`))
  ;[1 1 1] Get distances to all nav points
  (for _array_element (`local.Local Nav Points`)
    (`KismetArrayLibrary.Array_Add` (`local.Distances`) (`KismetMathLibrary.VSize` (- (`self.K2_GetActorLocation` _array_element) (`self.K2_GetActorLocation` (`self.Player`))))))
  ;[1 1 1] For loop for as many points are inside the nav point array
  (bind _output_get (set `local.For Loop Last Index` (`KismetArrayLibrary.Array_LastIndex` (`local.Local Nav Points`))))
  (for _ (range (+ _output_get 1))
    ;[1 1 1] Make new sorted array by continually finding the furthest point, adding it to the sorted array, then removing it from the other two
    (`KismetArrayLibrary.Array_Add` (`local.SortedNavs`) (`|GetArrayItem` (`local.Local Nav Points`) _indexofmaxvalue))
    (`KismetArrayLibrary.Array_Remove` (`local.Local Nav Points`) _indexofmaxvalue)
    (`KismetArrayLibrary.Array_Remove` (`local.Distances`) _indexofmaxvalue))
  ;[1 1 1] Reverse array so that lowest index is lowest length then return
  (`KismetArrayLibrary.Array_Reverse` _sortednavs)
  (return _sortednavs))

(fn `Get Random Location Within Nav Point`
  (params (NavPoint :type "/Game/Blueprints/BP_NavigationPoint Object Reference"))
  (returns (Location :type "Vector Structure"))
  (bind _returnvalue (`self.K2_GetActorLocation` NavPoint))
  (bind (_randomlocation _returnvalue_2) (`NavigationSystemV1.K2_GetRandomLocationInNavigableRadius` _returnvalue (`/Game/Blueprints/BP_NavigationPoint.Radius` NavPoint) null null))
  (if _returnvalue_2
    (return (+ _randomlocation (0.0 0.0 200.0)))
    (else
      (`KismetSystemLibrary.PrintString` "Did not successfullly Find Location")
      (return _returnvalue))))

(fn `Get References BeginPlay`
  (`|ExecutionSequence`
    (:`then_0`
      (bind _asbp_first_person_character (cast `/Game/Blueprints/BP_FirstPersonCharacter` (`GameplayStatics.GetPlayerCharacter` 0)))
      (bind _output_get (set `self.Player` _asbp_first_person_character))
      (set `self.Player Seeds` (`/Game/Blueprints/BP_FirstPersonCharacter.AC_SeedComponent` _output_get)))
    (:`then_1`
      (bind _outactors (`GameplayStatics.GetAllActorsOfClass` "/Game/Blueprints/BP_NavigationPoint.BP_NavigationPoint_C"))
      (set `self.NavPoints` _outactors))))

(fn `UserConstructionScript`)