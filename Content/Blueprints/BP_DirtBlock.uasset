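; Interactable farming dirt patch where the player plants a seed via a selection widget and keeps the crop watered.
; A DirtState switch drives interaction and Tick growth of Survive and Thrive meters, emptying the patch when a grown plant's Survive runs out.
; Looping timers move water from player to patch while interacting and drain it after planting.
; Sphere overlap toggles the water gauge for planted crops; crop production events are empty stubs.
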(event `self.ReceiveBeginPlay`
  (bind _player (`self.Player`))
  (`parent.ReceiveBeginPlay`)
  (set `self.Player Seeds` (`/Game/Blueprints/BP_FirstPersonCharacter.AC_SeedComponent` _player))
  (set `self.Player Water` (`/Game/Blueprints/BP_FirstPersonCharacter.AC_WaterComponent` _player))
  (bind _asw_plant_water (cast `/Game/Widgets/W_PlantWater` (`WidgetComponent.GetWidget` (`self.WaterWidget`))))
  (set `/Game/Widgets/W_PlantWater.DirtPatch` self _asw_plant_water))

(event `/Game/Blueprints/Interfaces/I_Interact.Release Interact`
  ;[1 1 1] Fill Water
  (`KismetSystemLibrary.K2_PauseTimerHandle` (stale `/Game/Blueprints/Interfaces/I_Interact.Interact` _returnvalue_2) :!label _label))

(event `/Game/Blueprints/Interfaces/I_Interact.Interact`
  (switch `/Game/Blueprints/Enums/E_DirtState` (`self.Dirt State`)
    (:`NewEnumerator0`
      (if (> (`/Game/Blueprints/Components/AC_SeedComponent.TotalSeeds` (`self.Player Seeds`)) 0)
        (bind _returnvalue (`|CreateWidget` "/Game/Widgets/W_SeedSelect.W_SeedSelect_C" null self))
        (`UserWidget.AddToViewport` _returnvalue 0)))
    (:`NewEnumerator1`
      ;[1 1 1] Fill Water
      (bind _returnvalue_2 (`KismetSystemLibrary.K2_SetTimerDelegate` (delegate `Water Crop`) 0.05 true :!label _label_2)))
    (:`NewEnumerator2`
      (goto _label_2))
    (:`NewEnumerator3`
      (goto _label_2))))

(event `Water Crop`
  ;[1 1 1] Fill Water
  (if (`self.Can Water`)
    (`/Engine/EditorBlueprintResources/StandardMacros.IsValid` (`/Game/Blueprints/BP_FirstPersonCharacter.InteractableActor` (`self.Player`))
      (:`Is Valid`
        (`/Game/Blueprints/Components/AC_WaterComponent.Update Water` (`self.Player Water`) (* (`self.WaterFillSpeed`) -1.0))
        (`/Game/Blueprints/Components/AC_WaterComponent.Update Water` (`self.AC_WaterComponent`) (`self.WaterFillSpeed`)))
      (:`Is Not Valid`
        (goto _label)))))

(event `Plant Seed`
  (params (SeedType :type "/Game/Blueprints/Enums/E_SeedTypes Enum" :default "NewEnumerator1"))
  ;[1 1 1] Plant Seed
  (bind _output_get (set `self.Crop Type` SeedType))
  (`/Game/Blueprints/Components/AC_SeedComponent.Remove Seed` (`self.Player Seeds`) _output_get)
  (`self.EnterNewDirtState` "NewEnumerator1"))

(event `StartWaterDrain`
  ;[1 1 1] Drain Water
  (bind _returnvalue (`KismetSystemLibrary.K2_SetTimerDelegate` (`|CreateDelegate` :!event `Water Drain`) 0.05 true)))

(event `Water Drain`
  ;[1 1 1] Drain Water
  (`/Game/Blueprints/Components/AC_WaterComponent.Update Water` (`self.AC_WaterComponent`) (`self.WaterDrainSpeed`)))

(event `self.Sphere.OnComponentBeginOverlap`
  (params (OverlappedComponent :type "PrimitiveComponent Object Reference") (OtherActor :type "Actor Object Reference") (OtherComp :type "PrimitiveComponent Object Reference") (OtherBodyIndex :type Integer) (bFromSweep :type Boolean) (SweepResult :type "HitResult Structure (by ref)"))
  ;[1 1 1] Show Gauges
  (if (`self.Check if Player and Planted` OtherActor)
    (`SceneComponent.SetHiddenInGame` (`self.WaterWidget`) false false)))

(event `StopWaterDrain`
  ;[1 1 1] Drain Water
  (`KismetSystemLibrary.K2_PauseTimerHandle` (stale `StartWaterDrain` _returnvalue)))

(event `self.Sphere.OnComponentEndOverlap`
  (params (OverlappedComponent :type "PrimitiveComponent Object Reference") (OtherActor :type "Actor Object Reference") (OtherComp :type "PrimitiveComponent Object Reference") (OtherBodyIndex :type Integer))
  ;[1 1 1] Show Gauges
  (if (`self.Check if Player and Planted` OtherActor)
    (`SceneComponent.SetHiddenInGame` (`self.WaterWidget`) true false)))

(event `StartCropProduction`)

(event `StopCropProduction`)

(event `self.ReceiveTick`
  (params (DeltaSeconds :type "Float (single-precision)"))
  ;[1 1 1] Event Tick
  (switch `/Game/Blueprints/Enums/E_DirtState` (`self.Dirt State`)
    (:`NewEnumerator1`
      (`self.GrowFirstTime`))
    (:`NewEnumerator2`
      (`self.ContinuedGrowth`))))

(fn `ContinuedGrowth`
  (bind _returnvalue (`self.ApplyGrowthOrDeath` (`KismetMathLibrary.SelectFloat` (`self.PlantSurvive`) (`self.PlantThrive`) (`/Game/Blueprints/Components/AC_WaterComponent.IsWaterZero` (`self.AC_WaterComponent`)))))
  ;[1 1 1] Check if Plant Survive Meter is Full
  (if (>= (`self.PlantSurvive`) (`self.SurviveMax`))
    ;[1 1 1] If Thrive is at 0, check if it should transition to survive or thrive, else then update thrive
    (if (<= (`self.PlantThrive`) 0.0)
      ;[1 1 1] Choose which value to update based on Water Supply
      (if (`/Game/Blueprints/Components/AC_WaterComponent.IsWaterZero` (`self.AC_WaterComponent`))
        ;[1 1 1] Set new value, and start or stop crop production accordingly
        (set `self.PlantSurvive` (`KismetMathLibrary.FClamp` _returnvalue 0.0 (`self.SurviveMax`)))
        (`self.StopCropProduction`)
        (else
          (set `self.PlantThrive` (`KismetMathLibrary.FClamp` _returnvalue 0.0 (`self.ThriveMax`)))
          (`self.StartCropProduction`)))
      (else
        ;[1 1 1] Update Thrive
        (set `self.PlantThrive` (`KismetMathLibrary.FClamp` (`self.ApplyGrowthOrDeath` (`self.PlantThrive`)) 0.0 (`self.ThriveMax`)))))
    (else
      ;[1 1 1] If it is not full, then alter Survive value based on Water Supply
      (bind _output_get (set `self.PlantSurvive` (`KismetMathLibrary.FClamp` (`self.ApplyGrowthOrDeath` (`self.PlantSurvive`)) 0.0 (`self.SurviveMax`))))
      ;[1 1 1] If Survive Meter is empty, then the plant dies, and the dirt patch becomes empty again
      (if (<= _output_get 0.0)
        (`self.EnterNewDirtState` "NewEnumerator0")))))

(fn `EnterNewDirtState`
  (params (`New State` :type "/Game/Blueprints/Enums/E_DirtState Enum" :default "NewEnumerator0"))
  (bind _output_get (set `self.Dirt State` `New State`))
  (switch `/Game/Blueprints/Enums/E_DirtState` _output_get
    (:`NewEnumerator0`
      (`SceneComponent.SetHiddenInGame` (`self.SM_BushSmall_A`) true false)
      (set `self.InteractText` "Water Plant")
      (`Widget.RemoveFromParent` (`/Game/Blueprints/BP_FirstPersonCharacter.InteractWidget` (`self.Player`)))
      (`SceneComponent.SetHiddenInGame` (`self.WaterWidget`) true false)
      (`self.StopWaterDrain`))
    (:`NewEnumerator1`
      (`SceneComponent.SetHiddenInGame` (`self.SM_BushSmall_A`) false false)
      (set `self.InteractText` "Water Plant")
      (`Widget.RemoveFromParent` (`/Game/Blueprints/BP_FirstPersonCharacter.InteractWidget` (`self.Player`)))
      (`SceneComponent.SetHiddenInGame` (`self.WaterWidget`) false false)
      (`self.StartWaterDrain`))))

(fn `GrowFirstTime`
  (if (>= (`self.PlantSurvive`) (`self.SurviveMax`))
    (`self.EnterNewDirtState` "NewEnumerator2")
    (else
      (set `self.PlantSurvive` (+ (`self.PlantSurvive`) (`KismetMathLibrary.SelectFloat` (* (`self.GrowthSpeed`) 2.0) (`self.GrowthSpeed`) (> (`/Game/Blueprints/Components/AC_WaterComponent.WaterLevel` (`self.AC_WaterComponent`)) 0.0))))
      (if (> (`self.PlantSurvive`) (`self.SurviveMax`))
        (set `self.PlantSurvive` (`self.SurviveMax`))))))

(fn `ReturnSurviveRatio`
  (returns (Ratio :type "Float (double-precision)"))
  (return (/ (`self.PlantSurvive`) (`self.SurviveMax`))))

(fn `ReturnThriveRatio`
  (returns (Ratio :type "Float (double-precision)"))
  (return (/ (`self.PlantThrive`) (`self.ThriveMax`))))

(fn `UserConstructionScript`
  (`parent.UserConstructionScript`)
  (bind _asw_plant_water (cast `/Game/Widgets/W_PlantWater` (`WidgetComponent.GetWidget` (`self.WaterWidget`))))
  (set `/Game/Widgets/W_PlantWater.DirtPatch` self _asw_plant_water))