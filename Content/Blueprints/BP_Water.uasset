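; BP_Water is an interactable water source that fills the player's water while the interact button is held.
; BeginPlay caches the player's ACWaterComponent, and Interact starts a looping quarter-second timer that calls AddWater on it.
; Releasing interact pauses the timer, as does a tick that finds the player's InteractableActor no longer valid.
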(event `self.ReceiveBeginPlay`
  (`parent.ReceiveBeginPlay`)
  (set `self.AC Water Component` (`/Game/Blueprints/BP_FirstPersonCharacter.AC_WaterComponent` (`self.Player`))))

(event `/Game/Blueprints/Interfaces/I_Interact.Release Interact`
  ;[1 1 1] Fill water as long as the interact button is held
  (`KismetSystemLibrary.K2_PauseTimerHandle` (stale `/Game/Blueprints/Interfaces/I_Interact.Interact` _returnvalue) :!label _label))

(event `/Game/Blueprints/Interfaces/I_Interact.Interact`
  ;[1 1 1] Fill water as long as the interact button is held
  (bind _returnvalue (`KismetSystemLibrary.K2_SetTimerDelegate` (delegate `Fill Water`) 0.25 true)))

(event `Fill Water`
  ;[1 1 1] Fill water as long as the interact button is held
  (`/Engine/EditorBlueprintResources/StandardMacros.IsValid` (`/Game/Blueprints/BP_FirstPersonCharacter.InteractableActor` (`self.Player`))
    (:`Is Valid`
      (`/Game/Blueprints/Components/AC_WaterComponent.Add Water` (`self.AC Water Component`)))
    (:`Is Not Valid`
      (goto _label))))

(fn `UserConstructionScript`
  (`parent.UserConstructionScript`))