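; BP_PotatoBarrel is an interactable barrel that takes potato seeds from the player until its countdown reaches zero.
; It runs on Interact or on the player's UseCrop dispatcher, which only checks that the player has a valid interactable, not that it is this barrel.
; With the matching crop equipped and seeds available, it removes a seed, decrements Counter, updates the count text and calls PotatoCounterIsZero at zero.
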(event `self.ReceiveBeginPlay`
  (bind _player (`self.Player`))
  (`parent.ReceiveBeginPlay`)
  (set `self.Player Seeds` (`/Game/Blueprints/BP_FirstPersonCharacter.AC_SeedComponent` _player))
  (add `/Game/Blueprints/BP_FirstPersonCharacter.Use Crop` _player (delegate `UseCropCall`)))

(event `UseCropCall`
  (`/Engine/EditorBlueprintResources/StandardMacros.IsValid` (`/Game/Blueprints/BP_FirstPersonCharacter.InteractableActor` (`self.Player`))
    (:`Is Valid`
      (`self.UseCropEvent`))))

(event `/Game/Blueprints/Interfaces/I_Interact.Interact`
  (bind _player_seeds (`self.Player Seeds`))
  (if (`|EnumEquality` (`/Game/Blueprints/BP_FirstPersonCharacter.EquippedCrop` (`self.Player`)) "NewEnumerator3") :!label _label
    (if (> (`self.Counter`) 0)
      (if (> (`/Game/Blueprints/Components/AC_SeedComponent.PotatoSeeds` _player_seeds) 0)
        (`/Game/Blueprints/Components/AC_SeedComponent.Remove Seed` _player_seeds "NewEnumerator3")
        (bind _result (`/Engine/EditorBlueprintResources/StandardMacros.DecrementInt` (`self.Counter`))
          (:`  `
            (`TextRenderComponent.K2_SetText` (`self.CountText`) (`KismetTextLibrary.Conv_IntToText` _result))
            (if (<= (`self.Counter`) 0)
              (`self.Potato Counter Is Zero`))))))))

(event `UseCropEvent`
  (goto _label))

(fn `UserConstructionScript`
  (`parent.UserConstructionScript`))