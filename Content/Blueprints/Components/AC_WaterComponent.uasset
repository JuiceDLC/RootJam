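; Actor component that tracks its owner's water level against a maximum, with zero and ratio queries.
; UpdateWater adds a clamped amount and triggers a player speed update call when the owner is the player character.
; DepleteWater decrements a truncated copy of the level, which does not appear to write back to WaterLevel.
; ReturnWaterRatio relies on WaterRatio, whose division node is left unused.
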(fn `Deplete Water`
  (params (NewParam :type Boolean))
  (if (> (`self.WaterLevel`) 0.0)
    (`/Engine/EditorBlueprintResources/StandardMacros.DecrementInt` (`KismetMathLibrary.FTrunc` (`self.WaterLevel`)))))

(fn `IsWaterZero`
  (returns (`Water is Zero` :type Boolean))
  (return (<= (`self.WaterLevel`) 0.0)))

(fn `Return Water Ratio`
  (returns (`Water Ratio` :type "Float (double-precision)"))
  (return (`self.WaterRatio`)))

(fn `Update Water`
  (params (`Water Amount` :type "Float (double-precision)"))
  (set `self.WaterLevel` (`KismetMathLibrary.FClamp` (+ `Water Amount` (`self.WaterLevel`)) 0.0 (`self.MaxWaterLevel`)))
  (if (== (`self.GetOwner`) (`GameplayStatics.GetPlayerCharacter` 0))
    (`self.UpdatePlayerSpeed`)))