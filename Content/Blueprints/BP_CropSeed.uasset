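; BP_CropSeed is an interactable crop seed pickup that gives the player a seed of its configured type.
; The construction script uses SeedType to set the sphere's material colour and the interaction text for carrot, onion, potato or garlic seeds.
; BeginPlay caches the player's seed component, and Interact adds the seed type to it before destroying the actor.
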(event `self.ReceiveBeginPlay`
  (`parent.ReceiveBeginPlay`)
  (set `self.Player Seeds` (`/Game/Blueprints/BP_FirstPersonCharacter.AC_SeedComponent` (`self.Player`))))

(event `/Game/Blueprints/Interfaces/I_Interact.Interact`
  (`/Game/Blueprints/Components/AC_SeedComponent.Add Seed` (`self.Player Seeds`) (`self.SeedType`))
  (`self.K2_DestroyActor`))

(fn `UserConstructionScript`
  (`parent.UserConstructionScript`)
  (`PrimitiveComponent.SetMaterial` (`self.Sphere`) 0 (select `/Game/Blueprints/Enums/E_SeedTypes` (`self.SeedType`) :`NewEnumerator0` "/Game/LevelPrototyping/Materials/MI_Solid_Orange.MI_Solid_Orange" :`NewEnumerator2` "/Game/LevelPrototyping/Materials/MI_Solid_Magenta.MI_Solid_Magenta" :`NewEnumerator3` "/Game/LevelPrototyping/Materials/MI_Solid_LightBrown.MI_Solid_LightBrown" :`NewEnumerator4` "/Game/LevelPrototyping/Materials/MI_Solid_LightPink.MI_Solid_LightPink" :!type "MaterialInterface Object Reference"))
  (set `self.InteractText` (select `/Game/Blueprints/Enums/E_SeedTypes` (`self.SeedType`) :`NewEnumerator0` "Carrot Seed" :`NewEnumerator2` "Onion Seed" :`NewEnumerator3` "Potato Seed" :`NewEnumerator4` "Garlic Seed")))